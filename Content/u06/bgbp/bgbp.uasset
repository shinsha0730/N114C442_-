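; Parallax background actor that shifts Far and Mid layer components as the player character moves along X.
; BeginPlay stores the player's starting X, and every Tick calls Up to measure the offset from it.
; Up sets each layer's relative location from a base position plus that offset scaled by its own factor (Farbg or Midbg), with fixed Y offsets separating the layers.
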(event EventBeginPlay
  (Variables|Default|Setpx (.X (Math|Vector|BreakVector (Transformation|GetActorLocation (Game|GetPlayerCharacter 0))))))

(event Collision|EventActorBeginOverlap
  (params (OtherActor :type Actor%20Object%20Reference)))

(event EventTick
  (params (DeltaSeconds :type Float%20%28single-precision%29))
  (CallFunction|Up))

(fn ConstructionScript)

(fn Up
  (Variables|Default|Setdx (- (.X (Math|Vector|BreakVector (Transformation|GetActorLocation (Game|GetPlayerCharacter 0)))) (Variables|Default|Getpx)))
  (Utilities|FlowControl|Sequence
    (:then_0
      (Transformation|SetRelativeLocation (Variables|Default|Getfar) (Math|Vector|MakeVector (+ (Variables|Default|Getxs) (* (Variables|Default|Getdx) (Variables|Default|Getfarbg))) (+ (Variables|Default|Getys) -2e+02) (Variables|Default|Getzs)) false false))
    (:then_1
      (Transformation|SetRelativeLocation (Variables|Default|Getmid) (Math|Vector|MakeVector (+ (Variables|Default|Getxs) (* (Variables|Default|Getdx) (Variables|Default|Getmidbg))) (+ (Variables|Default|Getys) -1e+02) (Variables|Default|Getzs)) false false))))