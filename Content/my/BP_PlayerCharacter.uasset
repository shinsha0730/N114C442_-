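; BP_PlayerCharacter is a side-scrolling player character that moves horizontally and jumps.
; On BeginPlay it registers an Enhanced Input mapping context, whose move action drives movement along world X and whose jump action starts and stops jumping.
; Movement is gated by a CanMove flag, printing a debug message when blocked.
; The input sign sets IsFacingRight, which flips PlayerSprite by rotating it 180 degrees.
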(event Input|EnhancedActionEvents|EnhancedInputActionIA_Move01
  (params (ActionValue :type Vector%202D%20Structure) (ElapsedSeconds :type Float%20%28double-precision%29) (TriggeredSeconds :type Float%20%28double-precision%29) (InputAction :type Input%20Action%20Object%20Reference :default "/Game/my/input/IA_Move01.IA_Move01"))
  (bind _x (Math|Vector2D|BreakVector2D ActionValue))
  (bind _playersprite (Variables|Default|GetPlayerSprite))
  (if (Variables|Default|GetCanMove)
    (if (> _x 0.0)
      (Variables|Default|SetisFacingRight true)
      (else
        (Variables|Default|SetisFacingRight false)))
    (Pawn|Input|AddMovementInput "1.000000,0.000000,0.000000" _x false)
    (if (Variables|Default|GetisFacingRight)
      (Transformation|SetRelativeRotation _playersprite "0, 0, 0" false false)
      (else
        (Transformation|SetRelativeRotation _playersprite "0.000000,180.000000,0.000000" false false)))
    (else
      (Development|PrintString "move looked"))))

(event Input|EnhancedActionEvents|EnhancedInputActionIA_Jump01
  (params (ActionValue :type Boolean) (ElapsedSeconds :type Float%20%28double-precision%29) (TriggeredSeconds :type Float%20%28double-precision%29) (InputAction :type Input%20Action%20Object%20Reference :default "/Game/my/input/IA_Jump01.IA_Jump01"))
  (:Started
    (Character|Jump))
  (:Completed
    (Character|StopJumping)))

(event EventBeginPlay
  (Input|AddMappingContext (PlayerController|LocalPlayerSubsystems|GetEnhancedInputLocalPlayerSubsystem (Game|GetPlayerController 0)) "/Game/my/input/IMC_Player01.IMC_Player01" 0 "(bIgnoreAllPressedKeysUntilRelease=True,bForceImmediately=False,bNotifyUserSettings=False)"))

(fn ConstructionScript)